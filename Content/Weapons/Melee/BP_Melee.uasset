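; BP_Melee is a base melee weapon Blueprint that runs montage-driven attack combos, with empty collision and combo start/end hooks for children.
; BeginPlay filters DataTable rows by MeleeType into MeleeDatas, which sets each step's montage, play rate, section and movability.
; Attack starts a combo or queues the next step while EnableNextCombo is set; PlayNextCombo advances it and Attacked resets it.
; SendDamage hits each actor once until OffCollision clears HittedActors.
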(event `self.ReceiveBeginPlay`
  ;[1 1 1] BeginPlay (DataTable 읽어오기)
  (`parent.ReceiveBeginPlay`)
  (bind _outrownames (`DataTableFunctionLibrary.GetDataTableRowNames` (`self.DataTable`)))
  (for _array_element _outrownames
    (bind _returnvalue (`|GetDataTableRow` (`self.DataTable`) _array_element)
      (:`then`
        (if (`|EnumEquality` (`.Type_14_C920C3B74B39CEDD3D98D9A25D1670AB` (break `/Game/Structs/FMeleeData` _returnvalue)) (`self.MeleeType`))
          (`KismetArrayLibrary.Array_Add` (`self.MeleeDatas`) _returnvalue))))))

(event `self.Attack`
  ;[1 1 1] Attack
  (`parent.Attack`) ; 왼쪽의 저 오버라이드 함수에서\n우클릭 -> 부모함수 클릭해서 만듬
  (if (`self.EnableNextCombo`)
    (set `self.EnableNextCombo` false)
    (set `self.ExsistNextCombo` true)
    (elif (`self.CanAttack`)
      (`self.SetStateAttacking`)
      (`self.PlayComboMontage`)
      (`self.StartCombo`))))

(event `PlayNextCombo`
  ;[1 1 1] Play Next Combo Montage
  (if (`self.ExsistNextCombo`)
    (set `self.ExsistNextCombo` false)
    (`/Engine/EditorBlueprintResources/StandardMacros.IncrementInt` (`self.ComboCount`)
      (:`  `
        (`self.PlayComboMontage`)
        (set `self.LastCombo` (== (- (`KismetArrayLibrary.Array_Length` (`self.MeleeDatas`)) 1) (`self.ComboCount`)))))))

(event `self.Attacked`
  ;[1 1 1] Attacked (End Attack)
  (`self.SetStateIdling`)
  (`self.SetStateMove` true)
  (set `self.ComboCount` 0)
  (set `self.EnableNextCombo` false)
  (set `self.LastCombo` false)
  (`self.EndCombo`))

(fn `EndCombo`)

(fn `OffCollision`
  (`KismetArrayLibrary.Array_Clear` (`self.HittedActors`)))

(fn `OnCollision`
  (params (CollisionType :type "/Game/Eunmerates/ECollisionType Enum" :default "NewEnumerator0")))

(fn `PlayComboMontage`
  (bind (_output_type _output_montage _output_playrate _output_startsectionname _output_canmove) (break `/Game/Structs/FMeleeData` (`|GetArrayItem` (`self.MeleeDatas`) (`self.ComboCount`))))
  (bind _ascharacter (cast `Character` (`self.GetOwner`)))
  (`Character.PlayAnimMontage` _ascharacter _output_montage _output_playrate _output_startsectionname)
  (`self.SetStateMove` _output_canmove))

(fn `SendDamage`
  (params (OtherActor :type "Actor Object Reference") (Damage :type "Float (double-precision)"))
  (returns (Result :type Boolean))
  (locals (FindActor :type Boolean))
  (for _array_element (`self.HittedActors`)
    (if (== _array_element (`local.OtherActor`))
      (set `local.FindActor` true) ; 로컬변수임
      (break)))
  (if (not (`local.FindActor`))
    (`KismetArrayLibrary.Array_Add` (`self.HittedActors`) (`local.OtherActor`))
    (bind _result (`parent.SendDamage` (`local.OtherActor`) (`local.Damage`)))
    (return _result)))

(fn `StartCombo`)

(fn `UserConstructionScript`
  (`parent.UserConstructionScript`))
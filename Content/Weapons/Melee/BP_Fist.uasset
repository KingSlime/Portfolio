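; BP_Fist is an unarmed melee weapon with hit spheres attached to hand and foot sockets on the owning Character's mesh.
; Collision overrides enable the sphere for the requested limb and disable all spheres when the hit window ends.
; Overlaps send damage scaled by combo count through WeaponPowerComponent, which is also notified when combos start and end.
; Separate events toggle slow motion through global time dilation.
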(event `self.ReceiveBeginPlay`
  (`parent.ReceiveBeginPlay`)
  (`self.AttachToSocket` (`self.LeftHand`) "Fist_LeftHand")
  (`self.AttachToSocket` (`self.RightHand`) "Fist_RightHand")
  (`self.AttachToSocket` (`self.LeftFoot`) "Fist_LeftFoot")
  (`self.AttachToSocket` (`self.RightFoot`) "Fist_RightFoot")
  (`self.SetCollision` "NoCollision"))

(event `self.OnCollision`
  (params (CollisionType :type "/Game/Eunmerates/ECollisionType Enum" :default "NewEnumerator0"))
  (`parent.OnCollision` CollisionType)
  (switch `/Game/Eunmerates/ECollisionType` CollisionType
    (:`NewEnumerator1`
      (`PrimitiveComponent.SetCollisionEnabled` (`self.LeftHand`) "QueryAndPhysics"))
    (:`NewEnumerator2`
      (`PrimitiveComponent.SetCollisionEnabled` (`self.RightHand`) "QueryAndPhysics"))
    (:`NewEnumerator3`
      (`PrimitiveComponent.SetCollisionEnabled` (`self.LeftFoot`) "QueryAndPhysics"))
    (:`NewEnumerator4`
      (`PrimitiveComponent.SetCollisionEnabled` (`self.RightFoot`) "QueryAndPhysics"))))

(event `self.OffCollision`
  (`parent.OffCollision`)
  (`self.SetCollision` "NoCollision"))

(event `self.LeftHand.OnComponentBeginOverlap`
  (params (OverlappedComponent :type "PrimitiveComponent Object Reference") (OtherActor :type "Actor Object Reference") (OtherComp :type "PrimitiveComponent Object Reference") (OtherBodyIndex :type Integer) (bFromSweep :type Boolean) (SweepResult :type "HitResult Structure (by ref)"))
  (bind _returnvalue (`/Game/Components/WeaponPowerComponent.GetComboPower` (`self.WeaponPowerComponent`) (`self.ComboCount`)))
  (`self.SendDamage` OtherActor _returnvalue))

(event `self.RightHand.OnComponentBeginOverlap`
  (params (OverlappedComponent :type "PrimitiveComponent Object Reference") (OtherActor :type "Actor Object Reference") (OtherComp :type "PrimitiveComponent Object Reference") (OtherBodyIndex :type Integer) (bFromSweep :type Boolean) (SweepResult :type "HitResult Structure (by ref)"))
  (bind _returnvalue (`/Game/Components/WeaponPowerComponent.GetComboPower` (`self.WeaponPowerComponent`) (`self.ComboCount`)))
  (`self.SendDamage` OtherActor _returnvalue))

(event `self.LeftFoot.OnComponentBeginOverlap`
  (params (OverlappedComponent :type "PrimitiveComponent Object Reference") (OtherActor :type "Actor Object Reference") (OtherComp :type "PrimitiveComponent Object Reference") (OtherBodyIndex :type Integer) (bFromSweep :type Boolean) (SweepResult :type "HitResult Structure (by ref)"))
  (bind _returnvalue (`/Game/Components/WeaponPowerComponent.GetComboPower` (`self.WeaponPowerComponent`) (`self.ComboCount`)))
  (`self.SendDamage` OtherActor _returnvalue))

(event `self.RightFoot.OnComponentBeginOverlap`
  (params (OverlappedComponent :type "PrimitiveComponent Object Reference") (OtherActor :type "Actor Object Reference") (OtherComp :type "PrimitiveComponent Object Reference") (OtherBodyIndex :type Integer) (bFromSweep :type Boolean) (SweepResult :type "HitResult Structure (by ref)"))
  (bind _returnvalue (`/Game/Components/WeaponPowerComponent.GetComboPower` (`self.WeaponPowerComponent`) (`self.ComboCount`)))
  (`self.SendDamage` OtherActor _returnvalue))

(event `self.StartCombo`
  (`parent.StartCombo`)
  (`/Game/Components/WeaponPowerComponent.StartAttack` (`self.WeaponPowerComponent`)))

(event `self.EndCombo`
  (`parent.EndCombo`)
  (`/Game/Components/WeaponPowerComponent.EndAttack` (`self.WeaponPowerComponent`)))

(event `StartSlowMotion`
  ;[1 1 1] SlowMotion
  (`GameplayStatics.SetGlobalTimeDilation` 0.25))

(event `EndSlowMotion`
  ;[1 1 1] SlowMotion
  (`GameplayStatics.SetGlobalTimeDilation` 1.0))

(fn `AttachToSocket`
  (params (Sphere :type "SphereComponent Object Reference") (SocketName :type Name))
  (bind _ascharacter (cast `Character` (`self.GetOwner`)))
  (`SceneComponent.K2_AttachToComponent` (`local.Sphere`) (`Character.Mesh` _ascharacter) (`local.SocketName`) "KeepRelative" "KeepRelative" "KeepRelative" true) ; 혹시 Sphere 안붙으면\nRoot씬컴포인가? 그 버전으로 선택할것
)

(fn `SetCollision`
  (params (CollisionType :type "ECollisionEnabled Enum" :default "NoCollision"))
  (for _array_element (`self.K2_GetComponentsByClass` "/Script/Engine.SphereComponent")
    (`PrimitiveComponent.SetCollisionEnabled` _array_element (`local.CollisionType`))))

(fn `UserConstructionScript`)
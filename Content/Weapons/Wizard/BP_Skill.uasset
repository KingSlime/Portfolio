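; BP_Skill is a base skill actor for the Wizard weapon, with Spell, Spelled and OffFocus events left empty, apparently for child skills to fill in.
; It resolves the wizard by casting its owner to BP_Wizard, then the character by casting that wizard's owner to Character.
; Gaining focus sends SetStateMoveMessage with true to that character; losing focus does nothing here.
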(event `Spell`)

(event `Spelled`)

(event `OnFocus`
  (message `/Game/Interfaces/IState.SetState_Move` (`self.GetWizardCharacter`) true))

(event `OffFocus`)

(fn `GetWizard`
  (returns (`AsBP Wizard` :type "/Game/Weapons/Wizard/BP_Wizard Object Reference"))
  (bind _asbp_wizard (cast `/Game/Weapons/Wizard/BP_Wizard` (`self.GetOwner`)))
  (return _asbp_wizard))

(fn `GetWizardCharacter`
  (returns (AsCharacter :type "Character Object Reference"))
  (bind _ascharacter (cast `Character` (`self.GetOwner` (`self.GetWizard`))))
  (return _ascharacter))

(fn `UserConstructionScript`)
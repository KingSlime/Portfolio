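; Wizard weapon Blueprint, extending a parent weapon, that casts one active skill from Heal, Warp and Throw.
; BeginPlay spawns all three skill actors, attaches them to the owning Character's mesh (Throw at a hand socket) and selects Heal.
; Attack and Attacked set spelling or idle state and forward to the active skill's Spell and Spelled.
; ChangeSkill and weapon selection events toggle each skill's focus.
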(event `self.ReceiveBeginPlay`
  (`parent.ReceiveBeginPlay`)
  (`|ExecutionSequence`
    (:`then_0`
      (bind _returnvalue (`|SpawnActorFromClass` "/Game/Weapons/Wizard/BP_Skill_Heal.BP_Skill_Heal_C" (`KismetMathLibrary.MakeTransform` (0.0 0.0 0.0)) "Undefined" "OverrideRootScale" self null))
      (set `self.Heal` _returnvalue) ; BP_SkillHeal 타입
      (bind _ascharacter (cast `Character` (`self.GetOwner`)))
      (`self.K2_AttachToComponent` (`self.Heal`) (`Character.Mesh` _ascharacter) "None" "KeepRelative" "KeepRelative" "KeepRelative" true) ; 메시 컴포에서 끌어 써야 함
    )
    (:`then_1`
      (bind _returnvalue_2 (`|SpawnActorFromClass` "/Game/Weapons/Wizard/BP_Skill_Warp.BP_Skill_Warp_C" (`KismetMathLibrary.MakeTransform` (0.0 0.0 0.0)) "Undefined" "OverrideRootScale" self null))
      (set `self.Warp` _returnvalue_2)
      (bind _ascharacter_2 (cast `Character` (`self.GetOwner`)))
      (`self.K2_AttachToComponent` (`self.Warp`) (`Character.Mesh` _ascharacter_2) "None" "KeepRelative" "KeepRelative" "KeepRelative" true))
    (:`then_2`
      (bind _returnvalue_3 (`|SpawnActorFromClass` "/Game/Weapons/Wizard/BP_Skill_Throw.BP_Skill_Throw_C" (`KismetMathLibrary.MakeTransform` (0.0 0.0 0.0)) "Undefined" "OverrideRootScale" self null))
      (set `self.Throw` _returnvalue_3)
      (bind _ascharacter_3 (cast `Character` (`self.GetOwner`)))
      (`self.K2_AttachToComponent` (`self.Throw`) (`Character.Mesh` _ascharacter_3) "Hand_Wizard" "KeepRelative" "KeepRelative" "KeepRelative" true))
    (:`then_3`
      (`self.ChangeSkill` (`self.Heal`)))))

(event `self.Attack`
  (`parent.Attack`)
  (if (and (`self.CanAttack`) (`KismetSystemLibrary.IsValid` (`self.Skill`)))
    (`self.SetStateSpelling`)
    (`/Game/Weapons/Wizard/BP_Skill.Spell` (`self.Skill`)) ; ..에서 재정의된 스펠 호출
  ))

(event `self.Attacked`
  (`parent.Attacked`)
  (`self.SetStateIdling`)
  (`/Game/Weapons/Wizard/BP_Skill.Spelled` (`self.Skill`)))

(event `self.OnSelected`
  (`/Engine/EditorBlueprintResources/StandardMacros.IsValid` (`self.Skill`)
    (:`Is Valid`
      (`/Game/Weapons/Wizard/BP_Skill.OnFocus` (`self.Skill`)))))

(event `self.OffSelected`
  (`/Engine/EditorBlueprintResources/StandardMacros.IsValid` (`self.Skill`)
    (:`Is Valid`
      (`/Game/Weapons/Wizard/BP_Skill.OffFocus` (`self.Skill`)))))

(fn `ChangeSkill`
  (params (NewSkill :type "/Game/Weapons/Wizard/BP_Skill Object Reference"))
  (if (!= NewSkill (`self.Skill`))
    (`/Engine/EditorBlueprintResources/StandardMacros.IsValid` (`self.Skill`)
      (:`Is Valid`
        (`/Game/Weapons/Wizard/BP_Skill.OffFocus` (`self.Skill`)) ; 사실상 매지볼의 핸드 파티클을 끄는 용도\n그 외에는 사용하는 곳이 없음
      )
      (:`Is Not Valid`
        _))
    (`/Engine/EditorBlueprintResources/StandardMacros.IsValid` (`local.NewSkill`)
      (:`Is Valid`
        (bind _output_get (set `self.Skill` (`local.NewSkill`))) ; 교체할 스킬로 바꿔 저장
        (`/Game/Weapons/Wizard/BP_Skill.OnFocus` _output_get))
      (:`Is Not Valid`
        (set `self.Skill` null)))))

(fn `UserConstructionScript`
  (`parent.UserConstructionScript`))
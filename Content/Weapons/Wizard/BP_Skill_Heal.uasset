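; BP_Skill_Heal is the Wizard's healing skill, overriding the Spell and Spelled events of its parent skill class.
; Spell calls the parent, disables the wizard's movement and plays the heal montage on the wizard character.
; Spelled calls the parent, re-enables movement and restores a fixed amount of health through the character's StatusComponent.
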(event `self.Spell`
  (`parent.Spell`)
  (`/Game/Weapons/BP_Weapon.SetStateMove` (`self.GetWizard`) false) ; 마법 중에는 이동 금지
  (`Character.PlayAnimMontage` (`self.GetWizardCharacter`) "/Game/Character/Montages/Wizard/MG_Heal_Montage.MG_Heal_Montage" 1.0 "None"))

(event `self.Spelled`
  (`parent.Spelled`)
  (`/Game/Weapons/BP_Weapon.SetStateMove` (`self.GetWizard`) true)
  (`/Game/Components/StatusComponent.IncreaseHealth` (`self.GetComponentByClass` (`self.GetWizardCharacter`) "/Game/Components/StatusComponent.StatusComponent_C") 20.0))

(fn `UserConstructionScript`
  (`parent.UserConstructionScript`))
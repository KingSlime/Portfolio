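; BP_ThrowItem is a short-lived thrown-item actor for the Wizard's throw skill, destroying itself after two seconds.
; It resolves its owner chain through BP_Skill_Throw up to BP_Wizard.
; Its BeginOverlap function routes damage on the hit actor through the wizard's SendDamage, spawns a supplied hit particle at an offset from that actor, then destroys the item.
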(event `self.ReceiveBeginPlay`
  (`self.SetLifeSpan` 2.0))

(fn `BeginOverlap`
  (params (OtherActor :type "Actor Object Reference") (HitParticle :type "ParticleSystem Object Reference") (Location :type "Vector Structure") (Damage :type "Float (double-precision)") (ParticleScale :type "Vector Structure"))
  (`/Game/Weapons/BP_Weapon.SendDamage` (`self.GetOwnerToWizard`) (`local.OtherActor`) (`local.Damage`))
  (`GameplayStatics.SpawnEmitterAtLocation` (`local.HitParticle`) (+ (`self.K2_GetActorLocation` (`local.OtherActor`)) (`local.Location`)) (struct) (`local.ParticleScale`))
  (`self.K2_DestroyActor`))

(fn `GetOwnerToThrow`
  (returns (`AsBP Skill Throw` :type "/Game/Weapons/Wizard/BP_Skill_Throw Object Reference"))
  (bind _asbp_skill_throw (cast `/Game/Weapons/Wizard/BP_Skill_Throw` (`self.GetOwner`)))
  (return _asbp_skill_throw))

(fn `GetOwnerToWizard`
  (returns (`AsBP Wizard` :type "/Game/Weapons/Wizard/BP_Wizard Object Reference"))
  (bind _asbp_wizard (cast `/Game/Weapons/Wizard/BP_Wizard` (`self.GetOwner` (`self.GetOwnerToThrow`))))
  (return _asbp_wizard))

(fn `UserConstructionScript`)
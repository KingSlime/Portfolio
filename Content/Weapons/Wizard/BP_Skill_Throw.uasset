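; Wizard skill that throws a selectable projectile, with a matching particle effect on the hand shown only while the skill is focused.
; Spell plays the throw montage, and a separate Throw event spawns the current item's actor at half scale from the hand socket, facing the wizard's yaw.
; ChangeItem looks up the given class in ThrowItems, stores its index for later throws and swaps the hand particle template to match.
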(event `self.ReceiveBeginPlay`
  (bind (_output_throwitemclass _output_attachparticle) (break `/Game/Structs/FThrowItem` (`|GetArrayItem` (`self.ThrowItems`) (`self.CurrentItem_Index`))))
  (`ParticleSystemComponent.SetTemplate` (`self.HandParticle`) _output_attachparticle)
  (`SceneComponent.SetVisibility` (`self.HandParticle`) false false))

(event `self.Spell`
  (`parent.Spell`)
  (`Character.PlayAnimMontage` (`self.GetWizardCharacter`) "/Game/Character/Montages/Wizard/MG_Throw_Montage.MG_Throw_Montage" 1.0 "None"))

(event `self.Spelled`
  (`parent.Spelled`))

(event `Throw`
  (bind _ascharacter (`self.GetWizardCharacter`))
  (bind (_returnvalue_roll _returnvalue_pitch _returnvalue_yaw) (`KismetMathLibrary.BreakRotator` (`self.K2_GetActorRotation` _ascharacter)))
  (bind _output_throwitemclass (break `/Game/Structs/FThrowItem` (`|GetArrayItem` (`self.ThrowItems`) (`self.CurrentItem_Index`))))
  (`|SpawnActorFromClass` _output_throwitemclass (`KismetMathLibrary.MakeTransform` (`SceneComponent.GetSocketLocation` (`Character.Mesh` _ascharacter) "Hand_ThrowItem") (`KismetMathLibrary.MakeRotator` 0.0 0.0 _returnvalue_yaw) (0.5 0.5 0.5)) "Undefined" "OverrideRootScale" self null))

(event `self.OnFocus`
  (`parent.OnFocus`)
  (`SceneComponent.SetVisibility` (`self.HandParticle`) true false))

(event `self.OffFocus`
  (`parent.OffFocus`)
  (`SceneComponent.SetVisibility` (`self.HandParticle`) false false))

(fn `ChangeItem`
  (params (NewClass :type "/Game/Weapons/Wizard/BP_ThrowItem Class Reference"))
  (locals (FindIndex :type Integer))
  (bind _output_throwitemclass (break `/Game/Structs/FThrowItem` (`|GetArrayItem` (`self.ThrowItems`) (`local.FindIndex`))))
  (bind (_output_throwitemclass_2 _output_attachparticle) (break `/Game/Structs/FThrowItem` (`|GetArrayItem` (`self.ThrowItems`) (`self.CurrentItem_Index`))))
  (for (_ _array_index) (`self.ThrowItems`)
    (set `local.FindIndex` _array_index) ; 증감자 i에 해당함
    (if (== _output_throwitemclass (`local.NewClass`))
      (break)))
  (set `self.CurrentItem_Index` (`local.FindIndex`))
  (`ParticleSystemComponent.SetTemplate` (`self.HandParticle`) _output_attachparticle))

(fn `UserConstructionScript`
  (`parent.UserConstructionScript`))
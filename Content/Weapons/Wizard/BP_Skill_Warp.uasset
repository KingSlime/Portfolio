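; Wizard warp skill that teleports the character to the floor point under the mouse cursor.
; GetCursorLocation traces WorldStatic objects and accepts only actors with "Floor" in their name, driving a decal and mesh preview while focused.
; Spell stores that point, locks movement and plays the warp montage, or calls Attacked on an invalid target.
; A separate Warp event performs the teleport, and Spelled restores movement.
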(event `self.ReceiveBeginPlay`
  (`parent.ReceiveBeginPlay`))

(event `self.Spell`
  (`parent.Spell`)
  (bind _location (`self.GetCursorLocation`)
    (:`True`
      (set `self.Location` _location) ; 픽킹이 Floor라면 위치 저장
      (set `self.Warpable` true)
      (`/Game/Weapons/BP_Weapon.SetStateMove` (`self.GetWizard`) false) ; 마법 중에는 이동 금지
      (`Character.PlayAnimMontage` (`self.GetWizardCharacter`) "/Game/Character/Montages/Wizard/MG_Warp_Montage.MG_Warp_Montage" 2.0 "None"))
    (:`False`
      (`/Game/Weapons/BP_Weapon.Attacked` (`self.GetWizard`)) ; 픽킹이 Floor가 아니라면 워프 종료
      (set `self.Warpable` false))))

(event `Warp`
  (if (`self.Warpable`)
    (set `self.Warpable` false)
    (`self.K2_SetActorLocation` (`self.GetWizardCharacter`) (`self.Location`) false true)))

(event `self.Spelled`
  (`parent.Spelled`)
  (`/Game/Weapons/BP_Weapon.SetStateMove` (`self.GetWizard`) true))

(event `self.ReceiveTick`
  (params (DeltaSeconds :type "Float (single-precision)"))
  (bind _decal (`self.Decal`))
  (bind _location (`self.GetCursorLocation`)
    (:`True`
      (`SceneComponent.K2_SetWorldLocation` _decal _location false false)
      (`SceneComponent.K2_SetWorldLocation` (`self.StaticMesh`) _location false false)
      (if (`self.Focus`)
        (`SceneComponent.SetVisibility` (`self.Decal`) true false)
        (`SceneComponent.SetVisibility` (`self.StaticMesh`) true false)))
    (:`False`
      (`SceneComponent.SetVisibility` _decal false false)
      (`SceneComponent.SetVisibility` (`self.StaticMesh`) false false))))

(event `self.OnFocus`
  (`parent.OnFocus`)
  (set `self.Focus` true))

(event `self.OffFocus`
  (`parent.OffFocus`)
  (set `self.Focus` false)
  (`SceneComponent.SetVisibility` (`self.Decal`) false false))

(fn `UserConstructionScript`
  (`parent.UserConstructionScript`))
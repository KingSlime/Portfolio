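; BP_GreatSwordMan is an enemy character that fights with a great sword, extending parent enemy events.
; On BeginPlay it spawns BP_GreateSword and attaches it to a holster socket on the mesh.
; Attach and Detach move the sword between hand and holster sockets, while Equipped and Unequipped update the current weapon and combat type.
; Taking damage stops its AI movement before the parent's damage handling runs.
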(event `self.ReceiveBeginPlay`
  (`parent.ReceiveBeginPlay`)
  (bind _returnvalue (`|SpawnActorFromClass` "/Game/Weapons/Melee/BP_GreateSword.BP_GreateSword_C" (`KismetMathLibrary.MakeTransform` (0.0 0.0 0.0)) "Undefined" "OverrideRootScale" self null)) ; 클래스에서 액터 스폰
  (bind _output_get (set `self.GreatSword` _returnvalue))
  (`self.K2_AttachToComponent` _output_get (`self.Mesh`) "Holster_GreatSword" "KeepRelative" "KeepRelative" "KeepRelative" true))

(event `self.Attach`
  (`parent.Attach`)
  (`self.K2_AttachToComponent` (`self.GreatSword`) (`self.Mesh`) "Hand_GreatSword" "KeepRelative" "KeepRelative" "KeepRelative" true))

(event `self.Detach`
  (`parent.Detach`)
  (`self.K2_AttachToComponent` (`self.GreatSword`) (`self.Mesh`) "Holster_GreatSword" "KeepRelative" "KeepRelative" "KeepRelative" true))

(event `self.Equipped`
  (`parent.Equipped`)
  (`self.Weapon_Change` (`self.GreatSword`))
  (set `self.CombatType` "NewEnumerator1"))

(event `self.Unequipped`
  (`parent.Unequipped`)
  (`self.Weapon_Change` null)
  (set `self.CombatType` "NewEnumerator0"))

(event `self.ReceiveAnyDamage`
  (params (Damage :type "Float (single-precision)") (DamageType :type "DamageType Object Reference") (InstigatedBy :type "Controller Object Reference") (DamageCauser :type "Actor Object Reference"))
  (`Controller.StopMovement` (`AIBlueprintHelperLibrary.GetAIController` self))
  (`parent.ReceiveAnyDamage` Damage DamageType InstigatedBy DamageCauser))

(fn `UserConstructionScript`
  (`parent.UserConstructionScript`))
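; BP_GrapplePointContainer is a trigger volume that manages which grapple points are available to the player inside it.
; When BP_Player enters the Box, it sets the player as each listed point's target and sends the player the whole array with a fixed activation distance.
; When the player leaves, it clears both the points' targets and the player's list, using message calls in both directions.
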(event `self.Box.OnComponentBeginOverlap`
  (params (OverlappedComponent :type "PrimitiveComponent Object Reference") (OtherActor :type "Actor Object Reference") (OtherComp :type "PrimitiveComponent Object Reference") (OtherBodyIndex :type Integer) (bFromSweep :type Boolean) (SweepResult :type "HitResult Structure (by ref)"))
  (bind _asbp_player (cast `/Game/Player/BP_Player` OtherActor))
  (for _array_element (`self.GrapplePoints`)
    (message `/Game/Interfaces/IGrapplePoint.SetGrapplePointTarget` _array_element _asbp_player))
  (message `/Game/Interfaces/IGrapplePointContainer.SetAllGrapplePointsInVolume` _asbp_player (`self.GrapplePoints`) 1800.0))

(event `self.Box.OnComponentEndOverlap`
  (params (OverlappedComponent :type "PrimitiveComponent Object Reference") (OtherActor :type "Actor Object Reference") (OtherComp :type "PrimitiveComponent Object Reference") (OtherBodyIndex :type Integer))
  (bind _asbp_player (cast `/Game/Player/BP_Player` OtherActor))
  (for _array_element (`self.GrapplePoints`)
    (message `/Game/Interfaces/IGrapplePoint.SetGrapplePointTarget` _array_element null))
  (message `/Game/Interfaces/IGrapplePointContainer.ClearAllGrapplePointsInVolume` _asbp_player))

(fn `UserConstructionScript`)
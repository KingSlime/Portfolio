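; BP_GrapplePoint is a grapple point object that tracks a state and the target actor, apparently the player, that selects it.
; SetGrapplePointTarget stores the passed Player and picks one of two enum states based on whether that reference is valid.
; CheckState applies a new state only when it differs, then calls OnGrapplePointStateChanged with itself and the state, while a getter exposes the current value.
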(event `self.SetGrapplePointTarget`
  (params (Player :type "/Game/Player/BP_Player Object Reference"))
  (bind _output_get (set `self.TargetActor` Player))
  (`/Engine/EditorBlueprintResources/StandardMacros.IsValid` _output_get
    (:`Is Valid`
      (`self.UpdateGrapplePointState` "NewEnumerator0") ; 요것도 냅다 붙여보자
    )
    (:`Is Not Valid`
      (`self.UpdateGrapplePointState` "NewEnumerator1"))))

(event `self.UpdateGrapplePointState`
  (params (NewState :type "/Game/Eunmerates/EGrapplePointType Enum" :default "NewEnumerator0"))
  (`self.CheckState` NewState))

(fn `CheckState`
  (params (NewState :type "/Game/Eunmerates/EGrapplePointType Enum" :default "NewEnumerator0"))
  (locals (PrevState :type "/Game/Eunmerates/EGrapplePointType Enum"))
  (set `local.PrevState` (`self.GrapplePointState`)) ; 로컬
  (if (`|EnumInequality` NewState (`self.GrapplePointState`))
    (set `self.GrapplePointState` (`local.NewState`))
    (`self.OnGrapplePointStateChanged` self (`self.GrapplePointState`))
    (else
      (set `self.GrapplePointState` (`local.PrevState`)))))

(fn `GetGrapplePointState`
  (returns (State :type "/Game/Eunmerates/EGrapplePointType Enum"))
  (return (`self.GrapplePointState`)))

(fn `UserConstructionScript`)
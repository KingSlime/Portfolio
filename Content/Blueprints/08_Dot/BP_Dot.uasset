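; BP_Dot is an actor that demonstrates the dot product as a way to measure angles to other actors.
; Every Tick it finds all StaticMeshActors and dots the normalized direction to each with its own up vector.
; It converts the result to degrees with arccosine and prints each angle to screen for a single frame.
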(event `self.ReceiveTick`
  (params (DeltaSeconds :type "Float (single-precision)"))
  (bind _outactors (`GameplayStatics.GetAllActorsOfClass` "/Script/Engine.StaticMeshActor"))
  (for _array_element _outactors
    (`KismetSystemLibrary.PrintString` (`KismetStringLibrary.Conv_DoubleToString` (`KismetMathLibrary.DegAcos` (`KismetMathLibrary.Dot_VectorVector` (`KismetMathLibrary.Normal` (- (`self.K2_GetActorLocation` _array_element) (`self.K2_GetActorLocation`))) (`self.GetActorUpVector`)))) true true (struct :`G` 0.66 :`B` 1.0 :`A` 1.0) 0.0)))

(fn `UserConstructionScript`)
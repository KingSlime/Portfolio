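; BP_Vector is a practice actor that demonstrates moving an actor with vector math through debug key presses.
; W raises it a small step along world Z.
; Q moves it along the forward vector of a fixed 45-degree yaw without rotating it, while E moves it along its own forward vector.
; Each press teleport-steps the location with SetActorLocation, without sweep, using normalized directions scaled by distance for Q and E.
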(event `Key|W`
  (params (Key :type "Key Structure"))
  ;[1 1 1] 1. W 눌러서 상승해보기
  (:`Pressed`
    (`self.K2_SetActorLocation` (+ (`self.K2_GetActorLocation`) (`KismetMathLibrary.MakeVector` 0.0 0.0 10.0)))))

(event `Key|Q`
  (params (Key :type "Key Structure"))
  ;[1 1 1] 2. Q키를 눌러서 45도 방향으로 이동(회전 없음)
  (:`Pressed`
    (`self.K2_SetActorLocation` (+ (`self.K2_GetActorLocation`) (* (`KismetMathLibrary.Normal` (`KismetMathLibrary.GetForwardVector` (`KismetMathLibrary.MakeRotator` 0.0 0.0 45.0))) 100.0)))))

(event `Key|E`
  (params (Key :type "Key Structure"))
  ;[1 1 1] 3. E키를 눌러서 액터의 전방 방향으로 이동하기
  (:`Pressed`
    (`self.K2_SetActorLocation` (+ (`self.K2_GetActorLocation`) (* (`KismetMathLibrary.Normal` (`KismetMathLibrary.GetForwardVector` (`self.K2_GetActorRotation`))) 100.0)))))

(fn `UserConstructionScript`)
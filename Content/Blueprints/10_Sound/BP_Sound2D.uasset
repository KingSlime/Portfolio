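; BP_Sound2D is a trigger actor that plays background music while the player is inside its static mesh volume.
; BeginPlay spawns BGM_Cue as a non-spatialized 2D sound, stores the audio component and immediately pauses it.
; Begin and end overlap events on the mesh, filtered to BP_Player, unpause and pause that component, so playback resumes where it stopped rather than restarting.
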(event `self.ReceiveBeginPlay`
  (bind _returnvalue (`GameplayStatics.SpawnSound2D` "/Game/Sounds/BGM_Cue.BGM_Cue" 1.0 1.0 0.0 null))
  (bind _output_get (set `self.Audio` _returnvalue))
  (`AudioComponent.SetPaused` _output_get true))

(event `self.StaticMesh.OnComponentBeginOverlap`
  (params (OverlappedComponent :type "PrimitiveComponent Object Reference") (OtherActor :type "Actor Object Reference") (OtherComp :type "PrimitiveComponent Object Reference") (OtherBodyIndex :type Integer) (bFromSweep :type Boolean) (SweepResult :type "HitResult Structure (by ref)"))
  (cast `/Game/Player/BP_Player` OtherActor)
  (`AudioComponent.SetPaused` (`self.Audio`) false))

(event `self.StaticMesh.OnComponentEndOverlap`
  (params (OverlappedComponent :type "PrimitiveComponent Object Reference") (OtherActor :type "Actor Object Reference") (OtherComp :type "PrimitiveComponent Object Reference") (OtherBodyIndex :type Integer))
  (cast `/Game/Player/BP_Player` OtherActor)
  (`AudioComponent.SetPaused` (`self.Audio`) true))

(fn `UserConstructionScript`)
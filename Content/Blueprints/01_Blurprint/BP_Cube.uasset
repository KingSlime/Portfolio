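; BP_Cube is a Blueprint that exercises variable arithmetic and on-screen debug printing.
; On BeginPlay it adds variables A and B into C and prints the result in red with a long display duration.
; On Tick it accumulates delta seconds into Time and prints the running total every frame.
; The construction script is empty.
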(event `self.ReceiveBeginPlay`
  (bind _output_get (set `self.C` (+ (`self.A`) (`self.B`))))
  (`KismetSystemLibrary.PrintString` (`KismetStringLibrary.Conv_IntToString` _output_get) true true (struct :`R` 1.0 :`A` 1.0) 30.0))

(event `self.ReceiveTick`
  (params (DeltaSeconds :type "Float (single-precision)"))
  (bind _output_get (set `self.Time` (+ DeltaSeconds (`self.Time`))))
  (`KismetSystemLibrary.PrintString` (`KismetStringLibrary.Conv_DoubleToString` _output_get)))

(fn `UserConstructionScript`)
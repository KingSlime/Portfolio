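; BP_Cube2 is an actor with a static mesh that moves steadily along the world Y axis and prints debug position info.
; BeginPlay prints the actor location, variable A in red, and a long-lasting line comparing the mesh's relative and world locations.
; Tick adds a MoveSpeed offset scaled by DeltaSeconds to the actor location without sweep, making movement frame-rate independent.
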(event `self.ReceiveBeginPlay`
  (bind _staticmesh (`self.StaticMesh`))
  (`KismetSystemLibrary.PrintString` (`KismetStringLibrary.Conv_VectorToString` (`self.K2_GetActorLocation`)))
  (`KismetSystemLibrary.PrintString` (`KismetStringLibrary.Conv_IntToString` (`self.A`)) true true (struct :`R` 1.0 :`A` 1.0) 1.0)
  (`KismetSystemLibrary.PrintString` (`KismetStringLibrary.Concat_StrStr` (`KismetSystemLibrary.GetDisplayName` self) " : " (`KismetStringLibrary.Conv_VectorToString` (`SceneComponent.RelativeLocation` _staticmesh)) " / " (`KismetStringLibrary.Conv_VectorToString` (`SceneComponent.K2_GetComponentLocation` _staticmesh))) true true (struct :`G` 0.66 :`B` 1.0 :`A` 1.0) 300.0))

(event `self.ReceiveTick`
  (params (DeltaSeconds :type "Float (single-precision)"))
  (`self.K2_SetActorLocation` (+ (`KismetMathLibrary.MakeVector` 0.0 (* DeltaSeconds (`self.MoveSpeed`))) (`self.K2_GetActorLocation`))))

(fn `UserConstructionScript`)
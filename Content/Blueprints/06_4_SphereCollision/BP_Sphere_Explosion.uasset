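; BP_Sphere_Explosion is an actor that sets off a one-shot radial blast at its location, pushing nearby physics bodies.
; Explosion runs a debug-drawn multi sphere trace for PhysicsBody objects, then applies a mass-scaled, constant-falloff radial impulse to each hit component and spawns a fire particle effect.
; A DoOnce gate blocks repeat blasts until the ExplosionReset event re-arms it.
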(event `Explosion`
  (bind _returnvalue (`self.K2_GetActorLocation`))
  (`/Engine/EditorBlueprintResources/StandardMacros.DoOnce` false :!label _label ; 리셋 경로로 들어오지 않는 한 한번만 실행되고 만다
    (:`Completed`
      (bind _outhits (`KismetSystemLibrary.SphereTraceMultiForObjects` :`Start` _returnvalue :`End` (+ _returnvalue (`KismetMathLibrary.MakeVector` 0.0 0.0 100.0)) :`Radius` 500.0 :`ObjectTypes` (`|MakeArray` "ObjectTypeQuery4" :!type "EObjectTypeQuery Enum") :`DrawDebugType` "ForDuration" :`DrawTime` 1.0))
      (for _array_element _outhits
        (bind (_bblockinghit _binitialoverlap _time _distance _location _impactpoint _normal _impactnormal _physmat _hitactor _hitcomponent) (`GameplayStatics.BreakHitResult` _array_element))
        (`PrimitiveComponent.AddRadialImpulse` _hitcomponent (`self.K2_GetActorLocation`) 500.0 (* (`PrimitiveComponent.GetMass` _hitcomponent) 500.0) "RIF_Constant" false))
      ;[1 1 1] 파티클 재생
      (`GameplayStatics.SpawnEmitterAtLocation` "/Game/Particles/Explosion/Fire_Exp_01.Fire_Exp_01" (`self.K2_GetActorLocation`)))))

(event `Explosion Reset`
  (goto _label :!via `Reset`))

(fn `UserConstructionScript`)
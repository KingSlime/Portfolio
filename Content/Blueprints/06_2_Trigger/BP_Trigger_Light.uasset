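; BP_Trigger_Light is a trigger actor that switches a point light on while another actor overlaps it.
; On BeginPlay it applies its Color variable to the PointLight component and hides the light.
; ActorBeginOverlap shows the light and ActorEndOverlap hides it again, with no filter on the overlapping actor and no overlap counting.
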(event `self.ReceiveBeginPlay`
  ;[1 1 1] 첨에 불끄기
  (`LightComponent.SetLightColor` (`self.PointLight`) (`self.Color`) true)
  (`SceneComponent.SetVisibility` (`self.PointLight`) false false))

(event `self.ReceiveActorBeginOverlap`
  (params (OtherActor :type "Actor Object Reference"))
  ;[1 1 1] 불켜기
  (`SceneComponent.SetVisibility` (`self.PointLight`) true false))

(event `self.ReceiveActorEndOverlap`
  (params (OtherActor :type "Actor Object Reference"))
  ;[1 1 1] 불끄기
  (`SceneComponent.SetVisibility` (`self.PointLight`) false false))

(fn `UserConstructionScript`)
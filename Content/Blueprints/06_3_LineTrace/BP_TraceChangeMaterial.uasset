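; Trace actor that randomizes the player character's material colors while the player crosses a line between two placed BP_TraceLine actors.
; BeginPlay gathers those actors and creates dynamic instances of the player's first two mesh materials, though the second SetMaterial has no material input.
; Tick draws the line and runs a Pawn object trace between them.
; ChangeColor randomizes BodyColor on both instances each frame BP_Player is hit.
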(event `self.ReceiveBeginPlay`
  (bind _mesh (`Character.Mesh` (`GameplayStatics.GetPlayerCharacter` 0)))
  (bind _outactors (`GameplayStatics.GetAllActorsOfClass` "/Game/Blueprints/06_3_LineTrace/BP_TraceLine.BP_TraceLine_C")) ; 화면상에 배치된 특정 타입의 객체들을 얻어와줌
  (set `self.Sphere` _outactors) ; 배열변수(우측 변수유형 오른쪽 색상버튼 클릭해서 배열화 가능)
  (bind _output_get (set `self.BodyMaterial` (`self.GetDynamicMaterial` 0))) ; 0번 엘레 인덱스를 DMI로 변환된 결과를 저장
  (`PrimitiveComponent.SetMaterial` _mesh 0 _output_get)
  (set `self.LogoMaterial` (`self.GetDynamicMaterial` 1))
  (`PrimitiveComponent.SetMaterial` _mesh 1 null))

(event `self.ReceiveTick`
  (params (DeltaSeconds :type "Float (single-precision)"))
  (bind _sphere (`self.Sphere`))
  (bind _sphere_2 (`self.Sphere`))
  (`KismetSystemLibrary.DrawDebugLine` (`self.K2_GetActorLocation` (`|GetArrayItem` _sphere)) (`self.K2_GetActorLocation` (`|GetArrayItem` _sphere 1)) (struct :`B` 1.0 :`A` 1.0))
  (bind (_outhit _returnvalue) (`KismetSystemLibrary.LineTraceSingleForObjects` (`self.K2_GetActorLocation` (`|GetArrayItem` _sphere_2)) (`self.K2_GetActorLocation` (`|GetArrayItem` _sphere_2 1)) (`|MakeArray` "ObjectTypeQuery3" :!type "EObjectTypeQuery Enum") false (`self.Sphere`) "ForOneFrame"))
  (`self.ChangeColor` _returnvalue _outhit) ; 커스텀이벤트 생성. 우상단 입력에서 파람 추가 가능
)

(event `ChangeColor`
  (params (Hitted :type Boolean) (HitDesc :type "HitResult Structure"))
  (bind _linearcolor (make `LinearColor` (`KismetMathLibrary.RandomFloatInRange` 0.0 1.0) (`KismetMathLibrary.RandomFloatInRange` 0.0 1.0) (`KismetMathLibrary.RandomFloatInRange` 0.0 1.0) 1.0))
  (if Hitted
    (cast `/Game/Player/BP_Player` (`.HitActor` (`GameplayStatics.BreakHitResult` HitDesc)))
    (`MaterialInstanceDynamic.SetVectorParameterValue` (`self.BodyMaterial`) "BodyColor" _linearcolor) ; 바디 머티리얼 색상 변경
    (`MaterialInstanceDynamic.SetVectorParameterValue` (`self.LogoMaterial`) "BodyColor" _linearcolor) ; 로고 머티리얼 색상 변경
  ))

(fn `GetDynamicMaterial`
  (params (`Element Index` :type Integer))
  (returns (ReturnValue :type "MaterialInstanceDynamic Object Reference"))
  (bind _returnvalue (`KismetMaterialLibrary.CreateDynamicMaterialInstance` (`PrimitiveComponent.GetMaterial` (`Character.Mesh` (`GameplayStatics.GetPlayerCharacter` 0)) (`local.Element Index`))))
  (return _returnvalue))

(fn `UserConstructionScript`)
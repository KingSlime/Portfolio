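; BP_Cross is a debug demo that visualizes the vector cross product between two referenced actors, A and B.
; Every Tick it draws arrows from A for the A-to-B offset (red), A's forward vector (green) and their cross product, forward × offset (blue).
; It also updates text with B's location, the cross result and the dot of A's forward and up vectors, which stays zero as they are perpendicular.
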(event `self.ReceiveTick`
  (params (DeltaSeconds :type "Float (single-precision)"))
  (bind _returnvalue (`self.Get_A_Location`))
  (bind _returnvalue_2 (`self.Get_A_Location`))
  (bind _returnvalue_3 (`self.Get_A_Location`))
  (bind _returnvalue_4 (`self.Get_A_Rotation`))
  (`|ExecutionSequence`
    (:`then_0`
      (`KismetSystemLibrary.DrawDebugArrow` _returnvalue (+ _returnvalue (`self.Get_AtoB_Location`)) 0.0 (struct :`R` 1.0 :`A` 1.0)))
    (:`then_1`
      (`KismetSystemLibrary.DrawDebugArrow` _returnvalue_2 (+ _returnvalue_2 (* (`KismetMathLibrary.GetForwardVector` (`self.Get_A_Rotation`)) 300.0)) 0.0 (struct :`G` 1.0 :`A` 1.0)))
    (:`then_2`
      (`KismetSystemLibrary.DrawDebugArrow` _returnvalue_3 (+ _returnvalue_3 (`KismetMathLibrary.Cross_VectorVector` (`KismetMathLibrary.GetForwardVector` (`self.Get_A_Rotation`)) (`self.Get_AtoB_Location`))) 0.0 (struct :`B` 1.0 :`A` 1.0)))
    (:`then_3`
      (`|ExecutionSequence`
        (:`then_0`
          (`TextRenderComponent.K2_SetText` (`self.PrintLocation`) (`KismetTextLibrary.Conv_StringToText` (`KismetStringLibrary.Concat_StrStr` "Location(B) : " (`KismetStringLibrary.Conv_VectorToString` (`self.K2_GetActorLocation` (`self.B`)))))))
        (:`then_1`
          (`TextRenderComponent.K2_SetText` (`self.PrintCross`) (`KismetTextLibrary.Conv_StringToText` (`KismetStringLibrary.Concat_StrStr` "Cross : " (`KismetStringLibrary.Conv_VectorToString` (`KismetMathLibrary.Cross_VectorVector` (`KismetMathLibrary.GetForwardVector` (`self.Get_A_Rotation`)) (`self.Get_AtoB_Location`)))))))
        (:`then_2`
          (`TextRenderComponent.K2_SetText` (`self.PrintDot`) (`KismetTextLibrary.Conv_StringToText` (`KismetStringLibrary.Concat_StrStr` "Dot : " (`KismetStringLibrary.Conv_DoubleToString` (`KismetMathLibrary.Dot_VectorVector` (`KismetMathLibrary.GetForwardVector` _returnvalue_4) (`KismetMathLibrary.GetUpVector` _returnvalue_4)))))))))))

(fn `Get_A_Location`
  (returns (ReturnValue :type "Vector Structure"))
  (return (`self.K2_GetActorLocation` (`self.A`))))

(fn `Get_A_Rotation`
  (returns (ReturnValue :type "Rotator Structure"))
  (return (`self.K2_GetActorRotation` (`self.A`))))

(fn `Get_AtoB_Location`
  (returns (ReturnValue :type "Vector Structure"))
  (return (- (`self.K2_GetActorLocation` (`self.B`)) (`self.Get_A_Location`))))

(fn `UserConstructionScript`)